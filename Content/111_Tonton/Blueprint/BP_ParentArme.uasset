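; BP_ParentArme is a parent weapon Blueprint that handles hitscan firing through its Tir and StopTir events.
; Tir plays a fire sound, line-traces forward from the mesh with debug drawing, and sends AttackMessage with damage and bleed (Hemoragie) to the hit actor.
; A delay-and-gate HoldInput macro separates taps from holds, but its outputs are empty.
; A shootWeapon multi-press counter macro is defined but unused here.
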(event `Tir`
  (bind _staticmesh (`self.StaticMesh`))
  (bind _returnvalue (`SceneComponent.K2_GetComponentLocation` _staticmesh))
  (`self.HoldInput` 0.0 :!label _label
    (:`Held`
      _)
    (:`Tapped`
      _))
  (`GameplayStatics.PlaySound2D` "/Game/SFX_OF_WEAPON/Fire/AudioCue/Weapon_Fire_14_Cue.Weapon_Fire_14_Cue" 1.0 1.0 0.0 null null)
  (bind (_outhit _returnvalue_2) (`KismetSystemLibrary.LineTraceSingle` :`Start` _returnvalue :`End` (+ _returnvalue (* (`SceneComponent.GetForwardVector` _staticmesh) (`self.Arme Distance`))) :`TraceChannel` "TraceTypeQuery4" :`DrawDebugType` "ForDuration"))
  (if _returnvalue_2
    (message `/Game/111_Tonton/Blueprint/BI_Interaction.attack` (`.HitActor` (`GameplayStatics.BreakHitResult` _outhit)) _outhit (`self.ArmeDegat`) (`self.Hemoragie ?`))))

(event `StopTir`
  (goto _label :!via `Released`))

(fn `UserConstructionScript`)