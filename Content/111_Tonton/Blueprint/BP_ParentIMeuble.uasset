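; Parent Blueprint for interactive furniture that holds an inventory (ArrayInventory) the player character BP_Tim can look through.
; A Box trigger enables input while BP_Tim overlaps it, then disables input and closes any open inventory when he leaves.
; The Use action toggles through a FlipFlop, either creating a UI_InventoryToilet widget for BP_Tim and showing the cursor, or removing that widget.
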(event `self.Box.OnComponentBeginOverlap`
  (params (OverlappedComponent :type "PrimitiveComponent Object Reference") (OtherActor :type "Actor Object Reference") (OtherComp :type "PrimitiveComponent Object Reference") (OtherBodyIndex :type Integer) (bFromSweep :type Boolean) (SweepResult :type "HitResult Structure (by ref)"))
  (cast `/Game/111_Tonton/Blueprint/BP_Tim` OtherActor)
  (`self.EnableInput` (`GameplayStatics.GetPlayerControllerFromID` 0)))

(event `self.Box.OnComponentEndOverlap`
  (params (OverlappedComponent :type "PrimitiveComponent Object Reference") (OtherActor :type "Actor Object Reference") (OtherComp :type "PrimitiveComponent Object Reference") (OtherBodyIndex :type Integer))
  (bind _asbp_tim (cast `/Game/111_Tonton/Blueprint/BP_Tim` OtherActor))
  (`self.DisableInput` (`GameplayStatics.GetPlayerControllerFromID` 0))
  (bind _inventaireuiref (`self.InventaireUIREF`)
    (:`then`
      (`/Game/111_Tonton/Blueprint/BP_Tim.CloseInventory` _asbp_tim _inventaireuiref))
    (:`else`)))

(event `InputAction|Use`
  (params (Key :type "Key Structure"))
  (:`Pressed`
    (`/Engine/EditorBlueprintResources/StandardMacros.FlipFlop`
      (:`A`
        (bind _asbp_tim (cast `/Game/111_Tonton/Blueprint/BP_Tim` (`GameplayStatics.GetPlayerCharacter` 0)))
        (bind _returnvalue (`|CreateWidget` "/Game/111_Tonton/UI/UI_InventoryToilet.UI_InventoryToilet_C"))
        (bind _output_get (set `self.InventaireUIREF` _returnvalue))
        (`/Game/111_Tonton/Blueprint/BP_Tim.LookInvotory` _asbp_tim (`self.ArrayInventory`) _output_get)
        (set `PlayerController.bShowMouseCursor` true (`GameplayStatics.GetPlayerControllerFromID` 0)))
      (:`B`
        (bind _inventaireuiref (`self.InventaireUIREF`)
          (:`then`
            (`Widget.RemoveFromParent` _inventaireuiref))
          (:`else`))))))

(fn `UserConstructionScript`)