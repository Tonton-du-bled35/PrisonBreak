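; Self-service tray point that hands a tray to the player (BP_Tim) or to prisoners entering its sphere.
; Tim's overlap passes a DoOnce, re-armed by the ResetDiner event, then sets the hand child actor to BP_Plateau and flags TakePlateau, unless ModeTravailSelf is active.
; Overlapping BP_Prisonnier actors skip the gate: they get TenirPlateau and the same tray class on their child actor.
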(event `ResetDiner`
  (goto _label :!via `Reset`))

(event `self.Sphere.OnComponentBeginOverlap`
  (params (OverlappedComponent :type "PrimitiveComponent Object Reference") (OtherActor :type "Actor Object Reference") (OtherComp :type "PrimitiveComponent Object Reference") (OtherBodyIndex :type Integer) (bFromSweep :type Boolean) (SweepResult :type "HitResult Structure (by ref)"))
  (bind _asbp_tim (cast `/Game/111_Tonton/Blueprint/BP_Tim` OtherActor)
    (:`then`
      (`/Engine/EditorBlueprintResources/StandardMacros.DoOnce` false :!label _label
        (:`Completed`
          (if (not (`/Game/111_Tonton/Blueprint/BP_Tim.ModeTravailSelf` _asbp_tim))
            (`ChildActorComponent.SetChildActorClass` (`/Game/111_Tonton/Blueprint/BP_Tim.ChildActorHand` _asbp_tim) "/Game/111_Tonton/Blueprint/Self/BP_Plateau.BP_Plateau_C")
            (bind _asbp_tim_2 (cast `/Game/111_Tonton/Blueprint/BP_Tim` (`GameplayStatics.GetPlayerPawn` 0)))
            (set `/Game/111_Tonton/Blueprint/BP_Tim.TakePlateau?` true _asbp_tim_2)))))
    (:`CastFailed`
      (bind _asbp_prisonnier (cast `/Game/111_Tonton/IA/BP_Prisonnier` OtherActor))
      (set `/Game/111_Tonton/IA/BP_Prisonnier.TenirPlateau?` true _asbp_prisonnier)
      (`ChildActorComponent.SetChildActorClass` (`/Game/111_Tonton/IA/BP_Prisonnier.ChildActor` _asbp_prisonnier) "/Game/111_Tonton/Blueprint/Self/BP_Plateau.BP_Plateau_C"))))

(fn `UserConstructionScript`)