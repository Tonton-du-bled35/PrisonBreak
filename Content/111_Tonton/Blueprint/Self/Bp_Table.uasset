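; Prison canteen table with four seats where the player and prisoners put down meal trays or sit.
; Use clears all trays in canteen work mode, otherwise places the player's tray at the hit seat's child actor.
; During meal time, seat collisions sit tray-carrying prisoners on free places and mark them taken.
; VerifPlace rebuilds the free-seat array from spawned trays; Tick prints each seat's state for debugging.
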(event `self.ReceiveBeginPlay`)

(event `/Game/111_Tonton/Blueprint/BI_Interaction.Use`
  (params (`Hit structure` :type "HitResult Structure"))
  (bind _asbp_tim (cast `/Game/111_Tonton/Blueprint/BP_Tim` (`GameplayStatics.GetPlayerCharacter` 0)))
  (if (`/Game/111_Tonton/Blueprint/BP_Tim.ModeTravailSelf` _asbp_tim)
    (`self.Netoyer Table`)
    (`/Game/111_Tonton/Blueprint/BP_Tim.FinirTravailSelf` _asbp_tim)
    (else
      (bind _indexplace (`self.select Place` `Hit structure`))
      (`self.Verif Place`)
      (`self.Prendre Place` _indexplace))))

(event `quit table`
  (bind _place_prise (`self.Place Prise`))
  (set `self.assis ?` false)
  (`KismetArrayLibrary.Array_Set` (`self.Place?`) _place_prise true)
  (`ChildActorComponent.SetChildActorClass` (`|GetArrayItem` (`self.PlacePlateau`) _place_prise) null))

(event `self.ReceiveTick`
  (params (DeltaSeconds :type "Float (single-precision)"))
  (for _array_element (`self.Place?`)
    (if _array_element
      (`KismetSystemLibrary.PrintString` "oui")
      (else
        (`KismetSystemLibrary.PrintString` "non")))))

(event `self.coll1.OnComponentBeginOverlap`
  (params (OverlappedComponent :type "PrimitiveComponent Object Reference") (OtherActor :type "Actor Object Reference") (OtherComp :type "PrimitiveComponent Object Reference") (OtherBodyIndex :type Integer) (bFromSweep :type Boolean) (SweepResult :type "HitResult Structure (by ref)"))
  (bind _place_ (`self.Place?`))
  (bind _asgm_level (cast `/Game/111_Tonton/Level/GM_Level` (`GameplayStatics.GetGameMode`)))
  (if (and (`|EnumEquality` (`/Game/111_Tonton/Level/GM_Level.comportement` _asgm_level) "NewEnumerator0") (`/Game/111_Tonton/Level/GM_Level.HeureManger?` _asgm_level))
    (bind _asbp_prisonnier (cast `/Game/111_Tonton/IA/BP_Prisonnier` OtherActor))
    (if (`/Game/111_Tonton/IA/BP_Prisonnier.TenirPlateau?` _asbp_prisonnier)
      (if (`|GetArrayItem` _place_)
        (`/Game/111_Tonton/IA/BP_Prisonnier.Assis` _asbp_prisonnier (`self.coll1`))
        (`KismetArrayLibrary.Array_Set` _place_)))))

(event `self.coll2.OnComponentBeginOverlap`
  (params (OverlappedComponent :type "PrimitiveComponent Object Reference") (OtherActor :type "Actor Object Reference") (OtherComp :type "PrimitiveComponent Object Reference") (OtherBodyIndex :type Integer) (bFromSweep :type Boolean) (SweepResult :type "HitResult Structure (by ref)"))
  (bind _place_ (`self.Place?`))
  (bind _asgm_level (cast `/Game/111_Tonton/Level/GM_Level` (`GameplayStatics.GetGameMode`)))
  (if (and (`|EnumEquality` (`/Game/111_Tonton/Level/GM_Level.comportement` _asgm_level) "NewEnumerator0") (`/Game/111_Tonton/Level/GM_Level.HeureManger?` _asgm_level))
    (bind _asbp_prisonnier (cast `/Game/111_Tonton/IA/BP_Prisonnier` OtherActor))
    (if (`/Game/111_Tonton/IA/BP_Prisonnier.TenirPlateau?` _asbp_prisonnier)
      (if (`|GetArrayItem` _place_ 1)
        (`/Game/111_Tonton/IA/BP_Prisonnier.Assis` _asbp_prisonnier (`self.coll2`))
        (`KismetArrayLibrary.Array_Set` _place_ 1)))))

(event `self.coll3.OnComponentBeginOverlap`
  (params (OverlappedComponent :type "PrimitiveComponent Object Reference") (OtherActor :type "Actor Object Reference") (OtherComp :type "PrimitiveComponent Object Reference") (OtherBodyIndex :type Integer) (bFromSweep :type Boolean) (SweepResult :type "HitResult Structure (by ref)"))
  (bind _place_ (`self.Place?`))
  (bind _asgm_level (cast `/Game/111_Tonton/Level/GM_Level` (`GameplayStatics.GetGameMode`)))
  (if (and (`|EnumEquality` (`/Game/111_Tonton/Level/GM_Level.comportement` _asgm_level) "NewEnumerator0") (`/Game/111_Tonton/Level/GM_Level.HeureManger?` _asgm_level))
    (bind _asbp_prisonnier (cast `/Game/111_Tonton/IA/BP_Prisonnier` OtherActor))
    (if (`/Game/111_Tonton/IA/BP_Prisonnier.TenirPlateau?` _asbp_prisonnier)
      (if (`|GetArrayItem` _place_ 2)
        (`/Game/111_Tonton/IA/BP_Prisonnier.Assis` _asbp_prisonnier (`self.coll3`))
        (`KismetArrayLibrary.Array_Set` _place_ 2)))))

(event `self.coll4.OnComponentBeginOverlap`
  (params (OverlappedComponent :type "PrimitiveComponent Object Reference") (OtherActor :type "Actor Object Reference") (OtherComp :type "PrimitiveComponent Object Reference") (OtherBodyIndex :type Integer) (bFromSweep :type Boolean) (SweepResult :type "HitResult Structure (by ref)"))
  (bind _place_ (`self.Place?`))
  (bind _asgm_level (cast `/Game/111_Tonton/Level/GM_Level` (`GameplayStatics.GetGameMode`)))
  (if (and (`|EnumEquality` (`/Game/111_Tonton/Level/GM_Level.comportement` _asgm_level) "NewEnumerator0") (`/Game/111_Tonton/Level/GM_Level.HeureManger?` _asgm_level))
    (bind _asbp_prisonnier (cast `/Game/111_Tonton/IA/BP_Prisonnier` OtherActor))
    (if (`/Game/111_Tonton/IA/BP_Prisonnier.TenirPlateau?` _asbp_prisonnier)
      (if (`|GetArrayItem` _place_ 3)
        (`/Game/111_Tonton/IA/BP_Prisonnier.Assis` _asbp_prisonnier (`self.coll4`))
        (`KismetArrayLibrary.Array_Set` _place_ 3)))))

(fn `Netoyer Table`
  (`ChildActorComponent.SetChildActorClass` (`self.Place03`) null)
  (`ChildActorComponent.SetChildActorClass` (`self.Place04`) null)
  (`ChildActorComponent.SetChildActorClass` (`self.Place01`) null)
  (`ChildActorComponent.SetChildActorClass` (`self.Place02`) null))

(fn `Prendre Place`
  (params (placePrise :type Integer))
  (bind _returnvalue (- placePrise 1))
  (if (!= _returnvalue -1)
    (if (`|GetArrayItem` (`self.Place?`) _returnvalue)
      (bind _asbp_tim (cast `/Game/111_Tonton/Blueprint/BP_Tim` (`GameplayStatics.GetPlayerCharacter` 0)))
      (if (`/Game/111_Tonton/Blueprint/BP_Tim.TakePlateau?` _asbp_tim)
        (`ChildActorComponent.SetChildActorClass` (`/Game/111_Tonton/Blueprint/BP_Tim.ChildActorHand` _asbp_tim) null)
        (`KismetArrayLibrary.Array_Set` (`self.Place?`) _returnvalue)
        (`ChildActorComponent.SetChildActorClass` (`|GetArrayItem` (`self.PlacePlateau`) _returnvalue) "/Game/111_Tonton/Blueprint/Self/BP_Plateau.BP_Plateau_C")))))

(fn `select Place`
  (params (hit :type "HitResult Structure"))
  (returns (IndexPlace :type Integer))
  (bind (_bblockinghit _binitialoverlap _time _distance _location _impactpoint _normal _impactnormal _physmat _hitactor _hitcomponent) (`GameplayStatics.BreakHitResult` hit))
  (if (== _hitcomponent (`self.coll1`))
    (set `self.IndexPlace` 1)
    (return (`self.IndexPlace`))
    (elif (== _hitcomponent (`self.coll2`))
      (set `self.IndexPlace` 2)
      (return (`self.IndexPlace`))
      (elif (== _hitcomponent (`self.coll3`))
        (set `self.IndexPlace` 3)
        (return (`self.IndexPlace`))
        (elif (== _hitcomponent (`self.coll4`))
          (set `self.IndexPlace` 4)
          (return (`self.IndexPlace`))
          (else
            (`KismetSystemLibrary.PrintString` "bug")))))))

(fn `UserConstructionScript`
  (set `self.PlacePlateau` (`|MakeArray` (`self.Place01`) (`self.Place02`) (`self.Place03`) (`self.Place04`)))
  (set `self.PlaceCollision` (`|MakeArray` (`self.coll1`) (`self.coll2`) (`self.coll3`) (`self.coll4`)))
  (`self.Verif Place`))

(fn `Verif Place`
  (for (_array_element _array_index) (`self.PlacePlateau`)
    (if (== (`ChildActorComponent.ChildActorClass` _array_element) "/Game/111_Tonton/Blueprint/Self/BP_Plateau.BP_Plateau_C")
      (`KismetArrayLibrary.Array_Set` (`self.Place?`) _array_index)
      (else
        (`KismetArrayLibrary.Array_Set` (`self.Place?`) _array_index true)))))