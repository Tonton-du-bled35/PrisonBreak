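; BP_Cuisinier is an AI-controlled cook that the player can interact with for money.
; On BeginPlay it has its AI controller run a behavior tree.
; Its Use event passes through a DoOnce, then adds a fixed sum to BP_Tim's Argent unless ResteTable is set.
; The DoOnce is never reset and precedes that check, so a blocked first use still consumes the reward.
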(event `self.ReceiveBeginPlay`
  (`AIController.RunBehaviorTree` (`AIBlueprintHelperLibrary.GetAIController` self) null))

(event `/Game/111_Tonton/Blueprint/BI_Interaction.Use`
  (params (`Hit structure` :type "HitResult Structure"))
  (`/Engine/EditorBlueprintResources/StandardMacros.DoOnce` false
    (:`Completed`
      (bind _asbp_tim (cast `/Game/111_Tonton/Blueprint/BP_Tim` (`GameplayStatics.GetPlayerCharacter` 0)))
      (if (not (`/Game/111_Tonton/Blueprint/BP_Tim.ResteTable?` _asbp_tim))
        (set `/Game/111_Tonton/Blueprint/BP_Tim.Argent` (+ (`/Game/111_Tonton/Blueprint/BP_Tim.Argent` _asbp_tim) 20.0) _asbp_tim)))))

(fn `UserConstructionScript`
  (`parent.UserConstructionScript`))