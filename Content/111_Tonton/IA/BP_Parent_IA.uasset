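; Parent AI character Blueprint handling health, death and a quest marker.
; QuetesView shows the Sims component while any quest flag is true.
; Attack subtracts weapon damage unless invulnerable, destroying the actor at zero health; hemorrhage hits start a timeline whose Pertedevie event drains life until Soinsrealiser stops it.
; Manger, SetRoles and the construction script are empty, and the Conportement switch is unconnected.
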(event `QuetesView`
  (params (`Liste quetes` :type "Array of Boolean"))
  (bind _sims (`self.sims`))
  ;[1 1 1] afficher ou pas le sims
  (set `self.Quete en cours ?` false)
  (for _array_element `Liste quetes`
    (if (== _array_element true)
      (set `self.Quete en cours ?` true)
      (break)))
  (if (`self.Quete en cours ?`)
    (`SceneComponent.SetVisibility` _sims true false)
    (else
      (`SceneComponent.SetVisibility` _sims false false))))

(event `Soinsrealiser`
  ;[1 1 1] Event Infliger degat
  (`Timeline|Timeline_0` :!via `Stop` :!label _label
    (:`pertedevie`
      (bind _result (`/Engine/EditorBlueprintResources/StandardMacros.DecrementFloat` (`.Vie_8_E940569D4343D7AD4E7E00A7CC09C563` (break `/Game/111_Tonton/Data/ST_Personnage` (`self.Structure`))))
        (:`  `
          (if (<= _result 0.0)
            (`self.Mourir`)))))))

(event `Manger`)

(event `/Game/111_Tonton/Blueprint/BI_Interaction.attack`
  (params (hit :type "HitResult Structure") (Degat_Arme :type "Float (single-precision)") (hemoragie :type Boolean))
  (bind (_nom _vie _gang _commerce_ _invulnerable_) (break `/Game/111_Tonton/Data/ST_Personnage` (`self.Structure`)))
  (bind _returnvalue (- _vie Degat_Arme))
  ;[1 1 1] Event Infliger degat
  (if _invulnerable_
    _
    (elif (<= _returnvalue 0.0)
      (`self.Mourir`)
      (else
        (set `self.Structure` (make `/Game/111_Tonton/Data/ST_Personnage` "" _returnvalue))
        (if hemoragie
          (goto _label :!via `PlayFromStart`))))))

(fn `Mourir`
  (`self.K2_DestroyActor`))

(fn `SetRoles`)

(fn `UserConstructionScript`)