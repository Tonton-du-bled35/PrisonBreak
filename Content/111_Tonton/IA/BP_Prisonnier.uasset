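; Prisoner NPC that runs a behavior tree, stores its spawn as its cell and shows its name.
; LoopClass fills a role list, drawing randomly before the last two branches add theirs; BeginPlay adds that class as a component.
; Use triggers the role's action, opens the interaction UI, halts AI, turns the prisoner and disables player input.
; Assis seats it by disabling gravity and collision, teleporting, stopping AI and flagging eating.
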(event `self.ReceiveBeginPlay`
  (`self.LoopClass`)
  (bind _returnvalue (`|AddComponentByClass` (`self.Class_0`)))
  (set `self.RoleREF` (cast `/Game/111_Tonton/Blueprint/Roles/BP_roleParent` _returnvalue :!pure true))
  (`AIController.RunBehaviorTree` (`AIBlueprintHelperLibrary.GetAIController` self) "/Game/111_Tonton/IA/BT_Prisionner.BT_Prisionner")
  (`BlackboardComponent.SetValueAsVector` (`AIBlueprintHelperLibrary.GetBlackboard` self) "cellulle" (`self.K2_GetActorLocation`))
  (`TextRenderComponent.K2_SetText` (`self.TextRender`) (`KismetTextLibrary.Conv_StringToText` (`.Nom_16_6BD2606340878A4BD4C96F8880A31BD5` (break `/Game/111_Tonton/Data/ST_Personnage` (`self.Structure`))))))

(event `/Game/111_Tonton/Blueprint/BI_Interaction.Use`
  (params (`Hit structure` :type "HitResult Structure"))
  ;[1 1 1] Action pour parler
  (`/Game/111_Tonton/Blueprint/Roles/BP_roleParent.Action1` (`self.RoleREF`) false)
  (set `PlayerController.bShowMouseCursor` true (`GameplayStatics.GetPlayerController` 0))
  (bind _returnvalue (`|CreateWidget` "/Game/111_Tonton/UI/UI_InteractionPrisonnier.UI_InteractionPrisonnier_C"))
  (bind _output_get (set `self.Ui InteractionPrisionnierREF` _returnvalue))
  (set `/Game/111_Tonton/UI/UI_InteractionPrisonnier.ParentREF` self _returnvalue)
  (`UserWidget.AddToViewport` _output_get 0)
  (`BrainComponent.StopLogic` (`AIController.BrainComponent` (`AIBlueprintHelperLibrary.GetAIController` self)) "")
  (bind _asbp_tim (cast `/Game/111_Tonton/Blueprint/BP_Tim` (`GameplayStatics.GetPlayerCharacter` 0)))
  (`self.K2_SetActorRelativeRotation` (`KismetMathLibrary.Conv_VectorToRotator` (* (`SceneComponent.GetForwardVector` (`Actor.RootComponent` _asbp_tim)) -1.0)))
  (`self.DisableInput` _asbp_tim (`GameplayStatics.GetPlayerController` 0)))

(event `OuvrirDialogue`)

(event `Commercer`)

(event `Assis`
  (params (`collision Actor` :type "SphereComponent Object Reference"))
  (`CharacterMovementComponent.SetMovementMode` (`self.CharacterMovement`) "MOVE_Flying" 0)
  (`PrimitiveComponent.SetEnableGravity` (`self.CapsuleComponent`) false)
  (`self.SetActorEnableCollision` false)
  (`self.K2_TeleportTo` (`SceneComponent.K2_GetComponentLocation` `collision Actor`) (`SceneComponent.K2_GetComponentRotation` `collision Actor`))
  (`BrainComponent.StopLogic` (`AIController.BrainComponent` (`AIBlueprintHelperLibrary.GetAIController` self)) "")
  (set `self.Manger?` true))

(fn `LoopClass`
  (`|ExecutionSequence`
    (:`then_0`
      (bind _asbp_role_1 (castclass `/Game/111_Tonton/Blueprint/Roles/BP_role1` null))
      (`KismetArrayLibrary.Array_Add` (`self. Roles`) _asbp_role_1)
      (set `self.Class_0` (`KismetArrayLibrary.Array_Random` (`self. Roles`))))
    (:`then_1`
      (bind _asbp_role_2 (castclass `/Game/111_Tonton/Blueprint/Roles/BP_role2` null))
      (`KismetArrayLibrary.Array_Add` (`self. Roles`) _asbp_role_2))
    (:`then_2`
      (bind _asbp_roles_3 (castclass `/Game/111_Tonton/Blueprint/Roles/BP_roles3` null))
      (`KismetArrayLibrary.Array_Add` (`self. Roles`) _asbp_roles_3))))

(fn `UserConstructionScript`
  (`parent.UserConstructionScript`)
  (`AddComponent|NODE_AddBP_RoleParent-1`))