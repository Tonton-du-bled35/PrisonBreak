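; GM_Level is a prison level manager that runs the in-game clock, controls cell doors and sets prisoner behaviour.
; Two seconds after BeginPlay it opens every BP_PrisonDooor and applies a starting behaviour, stored and written to each BP_Prisonnier's blackboard enum key "conportement".
; A self-recalling Clock event advances minutes and hours at a SpeedGame delay.
; A door-closing event exists but is not called here.
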(event `self.ReceiveBeginPlay`
  (`self.Clock`)
  (`KismetSystemLibrary.Delay` 2.0)
  (`self.OuvertureDesPortes`)
  (`self.Set Value Comportement` "NewEnumerator0"))

(event `OuvertureDesPortes`
  ;[1 1 1] OUverture/fermeture Des portes
  (bind _outactors (`GameplayStatics.GetAllActorsOfClass` "/Game/111_Tonton/Assets/Prop/BP_PrisonDooor.BP_PrisonDooor_C"))
  (for _array_element _outactors
    (`/Game/111_Tonton/Assets/Prop/BP_PrisonDooor.OuvrirPorte` _array_element)))

(event `FermetureDesPortes`
  ;[1 1 1] OUverture/fermeture Des portes
  (bind _outactors (`GameplayStatics.GetAllActorsOfClass` "/Game/111_Tonton/Assets/Prop/BP_PrisonDooor.BP_PrisonDooor_C"))
  (for _array_element _outactors
    (`/Game/111_Tonton/Assets/Prop/BP_PrisonDooor.FermerPorte` _array_element)))

(event `Clock`
  (`KismetSystemLibrary.Delay` (`self.SpeedGame`))
  (bind _result (`/Engine/EditorBlueprintResources/StandardMacros.IncrementInt` (`self.Minutes`))
    (:`  `
      (if (> _result 59)
        (set `self.Minutes` 0)
        (bind _result_2 (`/Engine/EditorBlueprintResources/StandardMacros.IncrementInt` (`self.Hours`))
          (:`  `
            (if (> _result_2 24)
              (set `self.Hours` 0)))))
      (`self.Clock`))))

(event `Set Value Comportement`
  (params (Conportement :type "/Game/111_Tonton/Data/E_Conportement Enum" :default "NewEnumerator0"))
  ;[1 1 1] Set comportement
  (set `self.comportement` Conportement)
  (bind _outactors (`GameplayStatics.GetAllActorsOfClass` "/Game/111_Tonton/IA/BP_Prisonnier.BP_Prisonnier_C"))
  (for _array_element _outactors
    (`BlackboardComponent.SetValueAsEnum` (`AIBlueprintHelperLibrary.GetBlackboard` _array_element) "conportement" Conportement)))

(fn `UserConstructionScript`)